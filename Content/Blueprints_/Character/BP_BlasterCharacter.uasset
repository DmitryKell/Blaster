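; BP_BlasterCharacter is the Blaster character Blueprint, with a ShowSniperScopeWidget event meant for the sniper scope overlay.
; The event body is empty, and the scope logic is disconnected, so it never runs.
; That unwired logic lazily creates WBP_SniperRifleScope, adds it to the viewport, then plays ScopeZoomIn forward to show or faster in reverse to hide.
; The construction script is empty.
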(event EventShowSniperScopeWidget
  (params (bShowWidget :type Boolean)))

(fn ConstructionScript)